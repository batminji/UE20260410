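; BP_Plane is a player-controlled plane pawn that constantly flies forward, steers by pitch and roll, and fires missiles.
; Tick feeds movement input along the forward vector, while the axis inputs apply frame-rate-independent local rotation.
; Fire spawns a BP_Missle at the Arrow component's transform.
; Holding Boost raises the movement scale, with separate timelines narrowing the camera field of view on press and widening it on release.
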(event EventTick
  (params (DeltaSeconds :type Float%20%28single-precision%29))
  (Pawn|Input|AddMovementInput (Transformation|GetActorForwardVector) (Variables|Default|GetMoveScale) false))

(event Input|ActionEvents|InputActionFire
  (params (Key :type Key%20Structure :default "None"))
  (:Pressed
    (Game|SpawnActorfromClass "/Game/Blueprints/BP_Missle.BP_Missle_C" (Transformation|GetWorldTransform (Variables|Default|GetArrow)) "Undefined" "MultiplyWithRoot" 0 0)))

(event Input|ActionEvents|InputActionBoost
  (params (Key :type Key%20Structure :default "None"))
  (:Pressed
    (Variables|Default|SetMoveScale (Variables|Default|GetMaxMoveScale))
    (bind _alpha (Timeline|TL_FieldOfView PlayFromStart)
      (:Update
        (Camera|SetFieldOfView (Variables|Default|GetCamera) (Math|Float|Lerp 9e+01 65.0 _alpha)))))
  (:Released
    (Variables|Default|SetMoveScale (Variables|Default|GetDefaultMoveScale))
    (bind _alpha_2 (Timeline|Timeline Play)
      (:Update
        (Camera|SetFieldOfView (Variables|Default|GetCamera) (Math|Float|Lerp 65.0 9e+01 _alpha_2))))))

(event Input|AxisEvents|InputAxisPitch
  (params (AxisValue :type Float%20%28single-precision%29))
  (Transformation|AddActorLocalRotation (Math|Rotator|MakeRotator 0.0 (* AxisValue (Utilities|Time|GetWorldDeltaSeconds) (Variables|Default|GetLookSpeed)) 0.0) false false))

(event Input|AxisEvents|InputAxisRoll
  (params (AxisValue :type Float%20%28single-precision%29))
  (Transformation|AddActorLocalRotation (Math|Rotator|MakeRotator (* AxisValue (Utilities|Time|GetWorldDeltaSeconds) (Variables|Default|GetTurnSpeed)) 0.0 0.0) false false))

(fn ConstructionScript)